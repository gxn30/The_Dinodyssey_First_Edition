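; Beetle actor that moves along the spline of a referenced track actor, starting on BeginPlay if flagged active.
; A timeline drives it from the spline's end back to its start, setting world location and rotation from the spline each update.
; Duration scales the timeline play rate, and a start offset sets the time at which playback begins.
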(event Custom|moveMovingObject
  (Components|Timeline|SetPlayRate (Variables|Default|GetmovingObjectMover) (/ 2e+01 (Variables|Default|Getduration)))
  (Components|Timeline|SetNewTime (Variables|Default|GetmovingObjectMover) (Variables|Default|GetmovingObjectStartOffset))
  (bind _alpha (Timeline|movingObjectMover Play)
    (:Update
      (Variables|Default|SetAlpha _alpha)
      (Transformation|SetActorLocationAndRotation (Spline|GetLocationatDistanceAlongSpline (Variables|/Game/1_dierenOverig/kever/bp_track_beetle_test1.bp_track_beetle_test1_C|GetusefulSpline (Variables|Default|GettrackRefKeverTest1)) (Math|Float|Lerp (Spline|GetSplineLength (Variables|/Game/1_dierenOverig/kever/bp_track_beetle_test1.bp_track_beetle_test1_C|GetusefulSpline (Variables|Default|GettrackRefKeverTest1))) 0.0 (Variables|Default|GetAlpha)) "World") (Spline|GetRotationatDistanceAlongSpline (Variables|/Game/1_dierenOverig/kever/bp_track_beetle_test1.bp_track_beetle_test1_C|GetusefulSpline (Variables|Default|GettrackRefKeverTest1)) (Math|Float|Lerp (Spline|GetSplineLength (Variables|/Game/1_dierenOverig/kever/bp_track_beetle_test1.bp_track_beetle_test1_C|GetusefulSpline (Variables|Default|GettrackRefKeverTest1))) 0.0 (Variables|Default|GetAlpha)) "World")))))

(event EventBeginPlay
  (if (Variables|Default|GetactiveMovingObject)
    (CallFunction|MoveMovingObject)))

(fn ConstructionScript)