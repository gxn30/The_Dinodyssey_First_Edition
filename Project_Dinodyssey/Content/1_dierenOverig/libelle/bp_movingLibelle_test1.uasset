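; Test Blueprint for a dragonfly (libelle) actor that moves along the spline of a referenced track actor, starting on BeginPlay when active.
; A timeline, with play rate scaled by a duration variable and start time set by an offset, drives an alpha from spline length toward zero.
; Each update sets world location and rotation from that distance, so rising alpha runs the spline in reverse.
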(event Custom|moveMovingObject
  (Components|Timeline|SetPlayRate (Variables|Default|GetmovingObjectMover) (/ 2e+01 (Variables|Default|Getduration)))
  (Components|Timeline|SetNewTime (Variables|Default|GetmovingObjectMover) (Variables|Default|GetmovingObjectStartOffset))
  (bind _alpha (Timeline|movingObjectMover Play)
    (:Update
      (Variables|Default|SetAlpha _alpha)
      (Transformation|SetActorLocationAndRotation (Spline|GetLocationatDistanceAlongSpline (Variables|/Game/1_dierenOverig/libelle/bp_track_Libelle_test1.bp_track_Libelle_test1_C|GetusefulSpline (Variables|Default|GettrackRefLibelleTest1)) (Math|Float|Lerp (Spline|GetSplineLength (Variables|/Game/1_dierenOverig/libelle/bp_track_Libelle_test1.bp_track_Libelle_test1_C|GetusefulSpline (Variables|Default|GettrackRefLibelleTest1))) 0.0 (Variables|Default|GetAlpha)) "World") (Spline|GetRotationatDistanceAlongSpline (Variables|/Game/1_dierenOverig/libelle/bp_track_Libelle_test1.bp_track_Libelle_test1_C|GetusefulSpline (Variables|Default|GettrackRefLibelleTest1)) (Math|Float|Lerp (Spline|GetSplineLength (Variables|/Game/1_dierenOverig/libelle/bp_track_Libelle_test1.bp_track_Libelle_test1_C|GetusefulSpline (Variables|Default|GettrackRefLibelleTest1))) 0.0 (Variables|Default|GetAlpha)) "World")))))

(event EventBeginPlay
  (if (Variables|Default|GetactiveMovingObject)
    (CallFunction|MoveMovingObject)))

(fn ConstructionScript)