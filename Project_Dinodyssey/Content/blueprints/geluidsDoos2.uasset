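; Sound box trigger that switches narrator ("verteller") audio through base sound mixes as the first-person player enters and leaves its volume.
; BeginPlay waits three seconds, then sets the master mute mix and plays a 2D cue.
; Overlap sets narrator 2 unmute and narrators 1 and 3 mute mixes in succession, each replacing the last; exit restores master mute.
; An unwired listener-range check is marked as not working.
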(event OnComponentBeginOverlap(muziekdoosTest2)
  (params (OverlappedComponent :type Primitive%20Component%20Object%20Reference) (OtherActor :type Actor%20Object%20Reference) (OtherComp :type Primitive%20Component%20Object%20Reference) (OtherBodyIndex :type Integer) (bFromSweep :type Boolean) (SweepResult :type Hit%20Result%20Structure%20%28by%20ref%29))
  (Utilities|Casting|CastToFirstPersonCharacter OtherActor)
  (Utilities|FlowControl|Sequence
    (:then_0
      (Class|GameplayStatics|SetBaseSoundMix "/Game/1_sounds/test/test_mixes/SCM_unmute_verteller2.SCM_unmute_verteller2"))
    (:then_1
      (Utilities|FlowControl|Sequence
        (:then_0
          (Class|GameplayStatics|SetBaseSoundMix "/Game/1_sounds/test/test_mixes/SCM_mute_verteller1.SCM_mute_verteller1"))
        (:then_1
          (Class|GameplayStatics|SetBaseSoundMix "/Game/1_sounds/test/test_mixes/SCM_mute_verteller3.SCM_mute_verteller3"))))))

(event OnComponentEndOverlap(muziekdoosTest2)
  (params (OverlappedComponent :type Primitive%20Component%20Object%20Reference) (OtherActor :type Actor%20Object%20Reference) (OtherComp :type Primitive%20Component%20Object%20Reference) (OtherBodyIndex :type Integer))
  (Utilities|Casting|CastToFirstPersonCharacter OtherActor)
  (Class|GameplayStatics|SetBaseSoundMix "/Game/1_sounds/test/test_mixes/SCM_mute_test1Master.SCM_mute_test1Master"))

(event EventBeginPlay
  (Utilities|FlowControl|Delay 3.0)
  (Class|GameplayStatics|SetBaseSoundMix "/Game/1_sounds/test/test_mixes/SCM_mute_test1Master.SCM_mute_test1Master")
  (Audio|PlaySound2D "/Game/1_sounds/test/test_audio/layton/r_sfc_circuit32_n_Cue.r_sfc_circuit32_n_Cue" 1.0 1.0 0.0 0 0)
  (Class|GameplayStatics|SetBaseSoundMix "/Game/1_sounds/test/test_mixes/SCM_mute_test1Master.SCM_mute_test1Master"))

(fn ConstructionScript)