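; Sound box Blueprint that unmutes what appears to be a second narrator track while the first-person player stands inside it.
; BeginPlay starts a cue at the actor's location, bracketed by two base sound mix changes that end on the master mute mix.
; Overlapping the Test3Muziekdoos2 component switches to the unmute mix and leaving restores the mute, each printing a debug string.
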(event OnComponentBeginOverlap(test3Muziekdoos2)
  (params (OverlappedComponent :type Primitive%20Component%20Object%20Reference) (OtherActor :type Actor%20Object%20Reference) (OtherComp :type Primitive%20Component%20Object%20Reference) (OtherBodyIndex :type Integer) (bFromSweep :type Boolean) (SweepResult :type Hit%20Result%20Structure%20%28by%20ref%29))
  (Utilities|Casting|CastToFirstPersonCharacter OtherActor)
  (Class|GameplayStatics|SetBaseSoundMix "/Game/1_sounds/test/test_mixes/SCM_unmute_verteller2.SCM_unmute_verteller2")
  (Development|PrintString "audio 2"))

(event OnComponentEndOverlap(test3Muziekdoos2)
  (params (OverlappedComponent :type Primitive%20Component%20Object%20Reference) (OtherActor :type Actor%20Object%20Reference) (OtherComp :type Primitive%20Component%20Object%20Reference) (OtherBodyIndex :type Integer))
  (Utilities|Casting|CastToFirstPersonCharacter OtherActor)
  (Class|GameplayStatics|SetBaseSoundMix "/Game/1_sounds/test/test_mixes/SCM_mute_test1Master.SCM_mute_test1Master")
  (Development|PrintString "einde 2"))

(event EventBeginPlay
  (Class|GameplayStatics|SetBaseSoundMix "/Game/1_sounds/test/test_mixes/SCM_mute_eersteSeconden.SCM_mute_eersteSeconden")
  (Audio|PlaySoundatLocation "/Game/1_sounds/test/test_audio/layton/r_sfc_circuit32_n_Cue.r_sfc_circuit32_n_Cue" (Transformation|GetActorLocation) "0, 0, 0" 1.0 1.0 0.0 0 0 0)
  (Class|GameplayStatics|SetBaseSoundMix "/Game/1_sounds/test/test_mixes/SCM_mute_test1Master.SCM_mute_test1Master"))

(fn ConstructionScript)