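; Sound box actor for a test level that toggles narrator audio ("verteller 3") through a trigger volume.
; On BeginPlay it plays a sound cue at its location, switching base sound mixes around it to start muted.
; Overlap begin applies the unmute mix and overlap end restores the master mute, with debug prints.
; Both handlers require the overlapping actor to pass chained casts to FirstPersonCharacter and the placeholder moving dino.
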(event OnComponentBeginOverlap(test4Muziekdoos3)
  (params (OverlappedComponent :type Primitive%20Component%20Object%20Reference) (OtherActor :type Actor%20Object%20Reference) (OtherComp :type Primitive%20Component%20Object%20Reference) (OtherBodyIndex :type Integer) (bFromSweep :type Boolean) (SweepResult :type Hit%20Result%20Structure%20%28by%20ref%29))
  (Utilities|Casting|CastToFirstPersonCharacter OtherActor)
  (Utilities|Casting|CastTotest1_placeholder_bewegendeDino OtherActor)
  (Class|GameplayStatics|SetBaseSoundMix "/Game/1_sounds/test/test_mixes/SCM_unmute_verteller3.SCM_unmute_verteller3")
  (Development|PrintString "audio 3")
  (Utilities|FlowControl|Delay 1.0)
  (Development|PrintString "hej dino"))

(event OnComponentEndOverlap(test4Muziekdoos3)
  (params (OverlappedComponent :type Primitive%20Component%20Object%20Reference) (OtherActor :type Actor%20Object%20Reference) (OtherComp :type Primitive%20Component%20Object%20Reference) (OtherBodyIndex :type Integer))
  (Utilities|Casting|CastToFirstPersonCharacter OtherActor)
  (Utilities|Casting|CastTotest1_placeholder_bewegendeDino OtherActor)
  (Class|GameplayStatics|SetBaseSoundMix "/Game/1_sounds/test/test_mixes/SCM_mute_test1Master.SCM_mute_test1Master")
  (Development|PrintString "einde 3")
  (Utilities|FlowControl|Delay 1.0)
  (Development|PrintString "doei dino"))

(event EventBeginPlay
  (Class|GameplayStatics|SetBaseSoundMix "/Game/1_sounds/test/test_mixes/SCM_mute_eersteSeconden.SCM_mute_eersteSeconden")
  (Audio|PlaySoundatLocation "/Game/1_sounds/test/test_audio/layton/n_daisy32_n_Cue.n_daisy32_n_Cue" (Transformation|GetActorLocation) "0, 0, 0" 1.0 1.0 0.0 0 0 0)
  (Class|GameplayStatics|SetBaseSoundMix "/Game/1_sounds/test/test_mixes/SCM_mute_test1Master.SCM_mute_test1Master"))

(fn ConstructionScript)