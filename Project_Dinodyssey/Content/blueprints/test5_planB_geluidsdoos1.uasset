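; A test sound-box trigger actor that switches narrator audio through sound mixes as the first-person character enters and leaves it.
; On BeginPlay it sets a mix that mutes the opening seconds and activates its audio component.
; Overlap begin sets the narrator unmute mix and overlap end sets a master mute mix, both printing debug messages.
; Casts to a placeholder moving dinosaur remain unwired.
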(event OnComponentBeginOverlap(test5_geluidsdoos1)
  (params (OverlappedComponent :type Primitive%20Component%20Object%20Reference) (OtherActor :type Actor%20Object%20Reference) (OtherComp :type Primitive%20Component%20Object%20Reference) (OtherBodyIndex :type Integer) (bFromSweep :type Boolean) (SweepResult :type Hit%20Result%20Structure%20%28by%20ref%29))
  (Utilities|Casting|CastToFirstPersonCharacter OtherActor)
  (Class|GameplayStatics|SetBaseSoundMix "/Game/1_sounds/test/test_mixes/SCM_unmute_verteller1.SCM_unmute_verteller1")
  (Development|PrintString "audio 1")
  (Utilities|FlowControl|Delay 1.0)
  (Development|PrintString "hej dino"))

(event OnComponentEndOverlap(test5_geluidsdoos1)
  (params (OverlappedComponent :type Primitive%20Component%20Object%20Reference) (OtherActor :type Actor%20Object%20Reference) (OtherComp :type Primitive%20Component%20Object%20Reference) (OtherBodyIndex :type Integer))
  (Utilities|Casting|CastToFirstPersonCharacter OtherActor)
  (Class|GameplayStatics|SetBaseSoundMix "/Game/1_sounds/test/test_mixes/SCM_mute_test1Master.SCM_mute_test1Master")
  (Development|PrintString "einde 1")
  (Utilities|FlowControl|Delay 1.0)
  (Development|PrintString "doei dino"))

(event EventBeginPlay
  (Utilities|FlowControl|Sequence
    (:then_0
      (Class|GameplayStatics|SetBaseSoundMix "/Game/1_sounds/test/test_mixes/SCM_mute_eersteSeconden.SCM_mute_eersteSeconden"))
    (:then_1
      (Components|Activation|Activate (Variables|Default|Getaudio5Doos1) false)
      (Development|PrintString "activatie 1" true true "(R=0.000000,G=0.660000,B=1.000000,A=1.000000)" 5.0))))

(fn ConstructionScript)